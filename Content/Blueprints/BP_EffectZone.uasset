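; BP_EffectZone is a zone actor that applies a configurable Gameplay Effect to living characters while they overlap it.
; On begin overlap it applies EffectClass through the character's own Ability System Component and stores the returned handle.
; On end overlap it removes one stack using that handle, a single variable shared by all overlapping characters.
; The construction script sets the zone's text label from Description and Color.
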(event Collision|EventActorEndOverlap
  (params (OtherActor :type Actor%20Object%20Reference))
  (bind _asscharacter_base (Utilities|Casting|CastToSCharacterBase OtherActor))
  (GameplayEffects|RemoveActiveGameplayEffect (Ability|GetAbilitySystemComponent _asscharacter_base) (Variables|Default|GetEffectHandle) 1))

(event Collision|EventActorBeginOverlap
  (params (OtherActor :type Actor%20Object%20Reference))
  (bind _asscharacter_base (Utilities|Casting|CastToSCharacterBase OtherActor))
  (if (and (Class|SCharacterBase|IsAlive _asscharacter_base) (Utilities|IsValid (Ability|GetAbilitySystemComponent _asscharacter_base)))
    (bind _returnvalue (GameplayEffects|ApplyGameplayEffectSpecToSelf (Ability|GetAbilitySystemComponent _asscharacter_base) (GameplayEffects|MakeOutgoingSpec (Ability|GetAbilitySystemComponent _asscharacter_base) (Variables|Default|GetEffectClass) 1.0 (GameplayEffects|MakeEffectContext (Ability|GetAbilitySystemComponent _asscharacter_base)))))
    (Variables|Default|SetEffectHandle _returnvalue)))

(fn ConstructionScript
  (bind _textrender (Variables|Default|GetTextRender))
  (Rendering|Components|TextRender|SetText _textrender (Variables|Default|GetDescription))
  (Rendering|Components|TextRender|SetTextRenderColor _textrender (Variables|Default|GetColor)))