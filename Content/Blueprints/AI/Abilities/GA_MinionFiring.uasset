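; Gameplay ability that makes an AI minion fire projectiles through a montage.
; A single-count repeat action plays the montage, and once that action finishes, any montage exit commits and ends the ability, so commit comes last.
; Montage.FireProjectile gameplay events spawn the projectile at the Muzzle_Front socket, aimed at the AI controller's focus actor or along control rotation without one.
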(event Ability|EventActivateAbility
  (bind _returnvalue (Ability|GetAvatarActorfromActorInfo))
  (bind _returnvalue_2 (Ability|GetAvatarActorfromActorInfo))
  (bind _aspawn (Utilities|Casting|CastToPawn _returnvalue))
  (bind _assenemy_character (Utilities|Casting|CastToSEnemyCharacter _returnvalue_2))
  (bind _returnvalue_3 (AI|GetAIController _assenemy_character))
  (bind _returnvalue_4 (Class|AIController|GetFocusActor _returnvalue_3))
  (Ability|Async|WaitGameplayEventToActor _returnvalue "(TagName=\"Montage.FireProjectile\")"
    (:then
      (bind _returnvalue_5 (Animation|GetPlayLength (Variables|Default|GetMontage%20to%20Play)))
      (|RepeatAction _returnvalue_5 1
        (:OnPerformAction
          (|PlayMontageandWaitProxy "None" (Variables|Default|GetMontage%20to%20Play) 1.0 "None" true 1.0 0.0
            (:OnCompleted
              _)
            (:OnBlendOut
              _)
            (:OnInterrupted
              _)
            (:OnCancelled
              _))
          (if (Variables|Default|GetEnds)
            (Ability|CommitAbility)
            (Ability|EndAbility)))
        (:OnFinished
          (Variables|Default|SetEnds true))))
    (:EventReceived
      (Game|SpawnActorfromClass (Variables|Default|GetProjectileClass) (Math|Transform|MakeTransform (Transformation|GetSocketLocation (Class|GameplayAbility|GetOwningComponentfromActorInfo) "Muzzle_Front") (Math|Rotator|SelectRotator (Math|Rotator|FindLookatRotation (Transformation|GetActorLocation _returnvalue_2) (Transformation|GetActorLocation _returnvalue_4)) (Pawn|GetControlRotation (.AsPawn (Utilities|Casting|CastToPawn (Ability|GetAvatarActorfromActorInfo))) :!class /Script/Engine.Pawn) (Utilities|IsValid _returnvalue_4))) "AlwaysSpawn" _aspawn _aspawn))))

(event Ability|EventOnEndAbility
  (params (bWasCancelled :type Boolean)))