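; Gameplay Ability for the AI Buff_Black charge melee attack that plays a montage and damages a nearby pawn.
; Once committed, it starts the current montage and advances the index, cycling through MontagesToPlay.
; The first Montage.Hit event triggers a sphere overlap at Muzzle_Front, applying DamageEffect to the first pawn found through that pawn's own ability system.
; The ability ends when the montage completes, blends out or is interrupted or cancelled.
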(event Ability|EventActivateAbility
  (bind _returnvalue (Ability|CommitAbility))
  (if _returnvalue
    (Utilities|FlowControl|Sequence
      (:then_0
        (|PlayMontageandWaitProxy "None" (Utilities|Array|Get(acopy) (Variables|Default|GetMontages%20to%20Play) (Variables|Default|GetCurrentMontageIndex)) 1.0 "None" true 1.0 0.0
          (:then
            (Ability|Async|WaitGameplayEventToActor (Ability|GetAvatarActorfromActorInfo) "(TagName=\"Montage.Hit\")" true
              (:EventReceived
                (bind (_outactors _returnvalue_2) (Collision|SphereOverlapActors (Transformation|GetSocketLocation (Class|GameplayAbility|GetOwningComponentfromActorInfo) "Muzzle_Front") 5e+02 (Utilities|Array|MakeArray "ObjectTypeQuery3") 0 (Utilities|Array|MakeArray (Ability|GetAvatarActorfromActorInfo))))
                (if _returnvalue_2
                  (GameplayEffects|ApplyGameplayEffectToSelf (Variables|/Script/Sorcerer.SCharacterBase|GetAbilitySystemComponent (.AsSCharacter%20Base (Utilities|Casting|CastToSCharacterBase (Utilities|Array|Get(acopy) _outactors)))) (Variables|Default|GetDamageEffect) 1.0 (GameplayEffects|MakeEffectContext (Variables|/Script/Sorcerer.SCharacterBase|GetAbilitySystemComponent (.AsSCharacter%20Base (Utilities|Casting|CastToSCharacterBase (Utilities|Array|Get(acopy) _outactors))))))))))
          (:OnCompleted
            (Ability|EndAbility :!label _label))
          (:OnBlendOut
            (goto _label))
          (:OnInterrupted
            (goto _label))
          (:OnCancelled
            (goto _label))))
      (:then_1
        (Variables|Default|SetCurrentMontageIndex (Math|Integer|%(Integer) (+ (Variables|Default|GetCurrentMontageIndex) 1) (Utilities|Array|Length (Variables|Default|GetMontages%20to%20Play))))))))

(event Ability|EventOnEndAbility
  (params (bWasCancelled :type Boolean)))