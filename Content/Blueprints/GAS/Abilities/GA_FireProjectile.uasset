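; Gameplay ability that fires a projectile in time with an attack montage.
; On activation it commits the ability, plays the montage, then waits for the Montage.FireProjectile gameplay event on the owning actor.
; That event spawns the projectile class at the Muzzle_01 socket, aimed along the pawn's control rotation with the pawn as instigator.
; The ability ends when the montage completes, blends out, or is interrupted or cancelled.
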(event Ability|EventActivateAbility
  (bind _returnvalue (Ability|GetOwningActorfromActorInfo))
  (bind _aspawn (Utilities|Casting|CastToPawn _returnvalue))
  (bind _returnvalue_2 (Ability|CommitAbility))
  (if _returnvalue_2
    (|PlayMontageandWaitProxy "None" (Variables|Sorcerer|Ability|GetMontage%20to%20Play) 1.0 "None" true 1.0 0.0
      (:then
        (Ability|Async|WaitGameplayEventToActor _returnvalue "(TagName=\"Montage.FireProjectile\")"
          (:EventReceived
            (Game|SpawnActorfromClass (Variables|Sorcerer|Ability|GetProjectileClass) (Math|Transform|MakeTransform (Transformation|GetSocketLocation (Class|GameplayAbility|GetOwningComponentfromActorInfo) "Muzzle_01") (Pawn|GetControlRotation _aspawn :!class /Script/Engine.Pawn)) "AlwaysSpawn" 0 _aspawn))))
      (:OnCompleted
        (Ability|EndAbility :!label _label))
      (:OnBlendOut
        (goto _label))
      (:OnInterrupted
        (goto _label))
      (:OnCancelled
        (goto _label)))))

(event Ability|EventOnEndAbility
  (params (bWasCancelled :type Boolean)))