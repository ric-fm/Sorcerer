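; Gameplay ability that plays a looping combo of attack montages, firing a projectile during attacks.
; Gameplay events drive it: SaveAttack opens the chain window, ResetCombo ends the ability, and FireProjectile spawns the projectile.
; Input is buffered through Pressed and Saved flags, so the next montage starts once both press and window have occurred, in either order.
; Projectiles spawn from the current attack's socket along the pawn's control rotation.
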(event Custom|SaveAttack
  (if (Variables|Default|GetPressed)
    (CallFunction|DoNextAttack)
    (else
      (Variables|Default|SetSaved true))))

(event Custom|ResetCombo
  (Development|PrintString "RESET COMBO")
  (Variables|Default|SetSaved false)
  (Ability|EndAbility))

(event Custom|DoAttack
  (Ability|Tasks|WaitInputPress false
    (:then
      (|PlayMontageandWaitProxy "None" (Utilities|Array|Get(acopy) (Variables|Sorcerer|Ability|GetMontages) (Variables|Default|GetCurrentAttackIndex)) 1.0 "None" true 1.0 0.0
        (:OnCompleted
          (Development|PrintString "completed"))
        (:OnBlendOut
          (Development|PrintString "blend out"))
        (:OnInterrupted
          (Development|PrintString "interrupted"))
        (:OnCancelled
          (Development|PrintString "cancelled"))))
    (:OnPress
      (CallFunction|InputPress))))

(event Custom|InputPress
  (if (Variables|Default|GetSaved)
    (CallFunction|DoNextAttack)
    (else
      (Variables|Default|SetPressed true))))

(event Custom|DoNextAttack
  (CallFunction|ClearHelpers)
  (bind _output_get (Variables|Default|SetCurrentAttackIndex (+ (Variables|Default|GetCurrentAttackIndex) 1)))
  (if (< _output_get (Utilities|Array|Length (Variables|Sorcerer|Ability|GetMontages)))
    _
    (else
      (Variables|Default|SetCurrentAttackIndex 0)))
  (CallFunction|DoAttack))

(event Custom|ClearHelpers
  (Variables|Default|SetPressed false)
  (Variables|Default|SetSaved false))

(event Custom|SpawnProjectile
  (bind _returnvalue (Ability|GetOwningActorfromActorInfo))
  (bind _aspawn (Utilities|Casting|CastToPawn _returnvalue))
  (Game|SpawnActorfromClass (Variables|Sorcerer|Ability|GetProjectileClass) (Math|Transform|MakeTransform (Transformation|GetSocketLocation (Class|GameplayAbility|GetOwningComponentfromActorInfo) (Utilities|Array|Get(acopy) (Variables|Sorcerer|Ability|GetSockets) (Variables|Default|GetCurrentAttackIndex))) (Pawn|GetControlRotation _aspawn :!class /Script/Engine.Pawn)) "AlwaysSpawn" 0 _aspawn))

(event Ability|EventActivateAbility
  (bind _returnvalue (Ability|CommitAbility))
  (if _returnvalue
    (Ability|Async|WaitGameplayEventToActor (Ability|GetOwningActorfromActorInfo) "(TagName=\"Montage.SaveAttack\")"
      (:then
        (Ability|Async|WaitGameplayEventToActor (Ability|GetOwningActorfromActorInfo) "(TagName=\"Montage.ResetCombo\")"
          (:then
            (Ability|Async|WaitGameplayEventToActor (Ability|GetOwningActorfromActorInfo) "(TagName=\"Montage.FireProjectile\")"
              (:then
                (CallFunction|DoAttack))
              (:EventReceived
                (CallFunction|SpawnProjectile)
                (Development|PrintString "spawn projectile"))))
          (:EventReceived
            (CallFunction|ResetCombo))))
      (:EventReceived
        (CallFunction|SaveAttack)))))

(event Ability|EventOnEndAbility
  (params (bWasCancelled :type Boolean))
  (Development|PrintString "PRIMARY PROJECTILE ENDED"))