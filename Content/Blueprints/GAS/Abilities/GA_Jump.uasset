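; GA_Jump is a Gameplay Ability that makes the avatar, an SCharacterBase, jump.
; Activation is allowed only when the avatar casts to that class and CanJump passes.
; After committing, it calls Jump and waits for input release, which cancels the ability; a failed commit ends it.
; Ending the ability calls StopJumping, so the jump lasts as long as input is held.
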(event Ability|EventActivateAbility
  (bind _returnvalue (Ability|CommitAbility))
  (if _returnvalue
    (Character|Jump (.AsSCharacter%20Base (Utilities|Casting|CastToSCharacterBase (Ability|GetAvatarActorfromActorInfo))))
    (Ability|Tasks|WaitInputRelease false
      (:OnRelease
        (Ability|CancelAbility)))
    (else
      (Ability|EndAbility))))

(event Ability|EventOnEndAbility
  (params (bWasCancelled :type Boolean))
  (Character|StopJumping (.AsSCharacter%20Base (Utilities|Casting|CastToSCharacterBase (Ability|GetAvatarActorfromActorInfo)))))

(fn K2CanActivateAbility
  (params (ActorInfo :type Gameplay%20Ability%20Actor%20Info%20Structure) (Handle :type Gameplay%20Ability%20Spec%20Handle%20Structure))
  (bind _avataractor (Utilities|Struct|BreakGameplayAbilityActorInfo ActorInfo))
  (bind (_asscharacter_base _bsuccess) (Utilities|Casting|CastToSCharacterBase _avataractor))
  (return "" (and _bsuccess (Character|CanJump _asscharacter_base))))