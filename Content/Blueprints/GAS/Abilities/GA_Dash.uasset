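; Gameplay Ability that dashes the player character along its last movement input vector, with a tiny upward bias.
; After committing, it applies a short constant root-motion force with gravity enabled and keeps the last root-motion velocity on finish.
; The ability ends when the force finishes or after a delay following input release, and immediately if commit fails.
; Activation is allowed only when the last input vector is non-zero.
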(event Ability|EventActivateAbility
  (bind _returnvalue (Ability|GetAvatarActorfromActorInfo))
  (bind _assplayer_character (Utilities|Casting|CastToSPlayerCharacter _returnvalue))
  (bind _charactermovement (Variables|/Script/Engine.Character|GetCharacterMovement _assplayer_character))
  (bind _returnvalue_2 (Ability|CommitAbility))
  (if _returnvalue_2
    (Ability|Tasks|ApplyRootMotionConstantForce "None" (+ (Pawn|Components|PawnMovement|GetLastInputVector _charactermovement) (Math|Vector|MakeVector 0.0 0.0 0.01)) 4e+03 0.5 false 0 "MaintainLastRootMotionVelocity" (Variables|/Script/Engine.MovementComponent|GetVelocity _charactermovement) 0.0 true
      (:then
        (Ability|Tasks|WaitInputRelease false
          (:OnRelease
            (Utilities|FlowControl|Delay 0.5))))
      (:OnFinish
        _))
    (Ability|EndAbility)
    (else
      (Ability|EndAbility))))

(event Ability|EventOnEndAbility
  (params (bWasCancelled :type Boolean)))

(fn K2CanActivateAbility
  (params (ActorInfo :type Gameplay%20Ability%20Actor%20Info%20Structure) (Handle :type Gameplay%20Ability%20Spec%20Handle%20Structure))
  (return "" (not (Math|Vector|VectorIsNearlyZero (Pawn|Components|PawnMovement|GetLastInputVector (Variables|/Script/Engine.Character|GetCharacterMovement (.AsSPlayer%20Character (Utilities|Casting|CastToSPlayerCharacter (.AvatarActor (Utilities|Struct|BreakGameplayAbilityActorInfo ActorInfo))))))))))