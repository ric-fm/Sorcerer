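; Gameplay ability for a hold-to-charge projectile that scales with hold time (clamped).
; If off cooldown, it starts a charging cue and montage while awaiting input release.
; Releasing past the minimum cast time commits, jumps to the "Shoot" section and applies a root-motion jump along current velocity; otherwise it cancels.
; A montage event clears the cue and takes muzzle-socket trace data, from which the server spawns the projectile along the player's aim.
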(event Ability|EventActivateAbility
  (bind _returnvalue (Ability|GetAvatarActorfromActorInfo))
  (bind _returnvalue_2 (Transformation|GetVelocity _returnvalue))
  (bind _returnvalue_3 (Class|GameplayAbility|CheckAbilityCooldown))
  (if _returnvalue_3
    (GameplayCue|AddGameplayCue :GameplayCueTag "(TagName=\"GameplayCue.Charging\")")
    (bind _timeheld (Ability|Tasks|WaitInputRelease false)
      (:then
        (|PlayMontageandWaitProxy "None" "/Game/Characters/Gideon/Montages/AM_Burden.AM_Burden" 1.0 "None" true 1.0 0.0
          (:then
            (Ability|Async|WaitGameplayEventToActor (Ability|GetAvatarActorfromActorInfo) "(TagName=\"Montage.FireProjectile\")"
              (:EventReceived
                (GameplayCue|RemoveGameplayCue "(TagName=\"GameplayCue.Charging\")")
                (bind _data (|WaitTargetData :TaskInstanceName "Test" :ConfirmationType "Instant" :Class "/Script/GameplayAbilities.GameplayAbilityTargetActor_SingleLineTrace" :MaxRange 1e+03 :TraceProfile "(Name=\"Projectile\")" :StartLocation (Utilities|Struct|MakeGameplayAbilityTargetingLocationInfo "SocketTransform" "0.000000,0.000000,0.000000|0.000000,0.000000,0.000000|1.000000,1.000000,1.000000" 0 (Class|GameplayAbility|GetOwningComponentfromActorInfo) 0 "Muzzle_01") :ReticleClass 0 :bDebug true)
                  (:ValidData
                    (Ability|HasAuthority
                      (:True
                        (Game|SpawnActorfromClass (Variables|Default|GetProjectileClass) (Math|Transform|MakeTransform (.TraceStart (Collision|BreakHitResult (Ability|TargetData|GetHitResultfromTargetData _data))) (Math|Rotator|MakeRotfromX (Class|SPlayerCharacter|GetAimingDirectionfrom (.AsSPlayer%20Character (Utilities|Casting|CastToSPlayerCharacter (Ability|GetAvatarActorfromActorInfo))) (.TraceStart (Collision|BreakHitResult (Ability|TargetData|GetHitResultfromTargetData _data))))) (Math|Vector|MakeVector (Math|Float|Clamp(Float) (Variables|Default|GetTime%20Held) 1.0 5.0) (Math|Float|Clamp(Float) (Variables|Default|GetTime%20Held) 1.0 5.0) (Math|Float|Clamp(Float) (Variables|Default|GetTime%20Held) 1.0 5.0))) "AlwaysSpawn" 0 (.AsPawn (Utilities|Casting|CastToPawn (Ability|GetAvatarActorfromActorInfo)))))))))))
          (:OnCompleted
            (Ability|EndAbility :!label _label))
          (:OnBlendOut
            (goto _label))
          (:OnInterrupted
            (goto _label))
          (:OnCancelled
            (goto _label))))
      (:OnRelease
        (if (> _timeheld (Variables|Default|GetMinCastingTime))
          (bind _returnvalue_4 (Ability|CommitAbility))
          (if _returnvalue_4
            (Variables|Default|SetTime%20Held _timeheld)
            (Ability|Animation|MontageJumptoSection "Shoot")
            (|ApplyRootMotionJumpForce "None" (Math|Rotator|MakeRotfromX _returnvalue_2) (Math|Vector|VectorLength _returnvalue_2) 3e+02 2.0 0.0 false "MaintainLastRootMotionVelocity" "0, 0, 0" 0.0)
            (else
              (Ability|CancelAbility :!label _label_2)))
          (else
            (goto _label_2)))))
    (else
      (Ability|EndAbility))))