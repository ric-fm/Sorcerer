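; Gameplay ability that grants a temporary sprint to SCharacterBase avatars, activatable only when the character is not falling.
; On activation it commits, adds the Travelling gameplay cue and boosts max walk speed.
; It ends after a positive Duration or, with StopOnInputRelease set, on input release, whichever comes first.
; Ending removes the cue and sets a hardcoded walk speed rather than restoring the previous one.
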(event Ability|EventActivateAbility
  (bind _duration (Variables|Sorcerer|Ability|GetDuration))
  (Ability|CommitAbility)
  (GameplayCue|AddGameplayCue :GameplayCueTag "(TagName=\"GameplayCue.Travelling\")")
  (Variables|/Script/Engine.CharacterMovementComponent|SetMaxWalkSpeed (Variables|/Script/Engine.Character|GetCharacterMovement (.AsSCharacter%20Base (Utilities|Casting|CastToSCharacterBase (Ability|GetAvatarActorfromActorInfo)))) 5e+03)
  (if (Variables|Default|GetStopOnInputRelease)
    (Ability|Tasks|WaitInputRelease false
      (:then
        (if (> _duration 0.0) :!label _label
          (Utilities|FlowControl|Delay _duration)
          (Ability|EndAbility)))
      (:OnRelease
        (Ability|EndAbility)))
    (else
      (goto _label))))

(event Ability|EventOnEndAbility
  (params (bWasCancelled :type Boolean))
  (GameplayCue|RemoveGameplayCue "(TagName=\"GameplayCue.Travelling\")")
  (Variables|/Script/Engine.CharacterMovementComponent|SetMaxWalkSpeed (Variables|/Script/Engine.Character|GetCharacterMovement (.AsSCharacter%20Base (Utilities|Casting|CastToSCharacterBase (Ability|GetAvatarActorfromActorInfo)))) 1e+03))

(fn K2CanActivateAbility
  (params (ActorInfo :type Gameplay%20Ability%20Actor%20Info%20Structure) (Handle :type Gameplay%20Ability%20Spec%20Handle%20Structure))
  (return "" (not (AI|Components|NavMovement|IsFalling (Variables|/Script/Engine.Character|GetCharacterMovement (.AsSCharacter%20Base (Utilities|Casting|CastToSCharacterBase (.AvatarActor (Utilities|Struct|BreakGameplayAbilityActorInfo ActorInfo)))))))))