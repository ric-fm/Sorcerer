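; Gameplay ability that chains attack montages and fires projectiles for as long as the input is held.
; Montage.FireProjectile events spawn ProjectileClass at the socket matching the current attack, aimed via SPlayerCharacter's aiming direction.
; Montage.SaveAttack events advance to the next montage, wrapping around, or end the ability once input release has cleared ContinueFiring.
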(event Custom|SaveAttack
  (if (Variables|Default|GetContinueFiring)
    (CallFunction|DoNextAttack)
    (else
      (Ability|EndAbility))))

(event Custom|DoAttack
  (|PlayMontageandWaitProxy "None" (Utilities|Array|Get(acopy) (Variables|Sorcerer|Ability|GetMontages) (Variables|Default|GetCurrentAttackIndex)) 1.0 "None" true 1.0 0.0))

(event Custom|DoNextAttack
  (bind _output_get (Variables|Default|SetCurrentAttackIndex (+ (Variables|Default|GetCurrentAttackIndex) 1)))
  (if (< _output_get (Utilities|Array|Length (Variables|Sorcerer|Ability|GetMontages)))
    _
    (else
      (Variables|Default|SetCurrentAttackIndex 0)))
  (CallFunction|DoAttack))

(event Custom|SpawnProjectile
  (bind _returnvalue (Class|GameplayAbility|GetOwningComponentfromActorInfo))
  (bind _sockets (Variables|Sorcerer|Ability|GetSockets))
  (bind _currentattackindex (Variables|Default|GetCurrentAttackIndex))
  (bind _output (Utilities|Array|Get(acopy) _sockets _currentattackindex))
  (bind _returnvalue_2 (Transformation|GetSocketLocation _returnvalue _output))
  (Game|SpawnActorfromClass (Variables|Sorcerer|Ability|GetProjectileClass) (Math|Transform|MakeTransform _returnvalue_2 (Math|Rotator|MakeRotfromX (Class|SPlayerCharacter|GetAimingDirectionfrom (.AsSPlayer%20Character (Utilities|Casting|CastToSPlayerCharacter (Ability|GetAvatarActorfromActorInfo))) _returnvalue_2))) "AlwaysSpawn" 0 (.AsPawn (Utilities|Casting|CastToPawn (Ability|GetOwningActorfromActorInfo)))))

(event Ability|EventActivateAbility
  (bind _returnvalue (Ability|CommitAbility))
  (if _returnvalue
    (Ability|Async|WaitGameplayEventToActor (Ability|GetOwningActorfromActorInfo) "(TagName=\"Montage.SaveAttack\")"
      (:then
        (Ability|Async|WaitGameplayEventToActor (Ability|GetOwningActorfromActorInfo) "(TagName=\"Montage.FireProjectile\")"
          (:then
            (CallFunction|DoAttack)
            (Ability|Tasks|WaitInputRelease false
              (:OnRelease
                (Variables|Default|SetContinueFiring false))))
          (:EventReceived
            (CallFunction|SpawnProjectile))))
      (:EventReceived
        (CallFunction|SaveAttack)))))